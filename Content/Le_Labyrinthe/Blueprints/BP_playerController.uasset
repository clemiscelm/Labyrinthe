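; Player controller for Le_Labyrinthe that handles first-person movement and camera look through Enhanced Input.
; On BeginPlay it adds the IMC_Inputs mapping context to the local player subsystem.
; IA_move drives a BP_FirstPersonCharacter found with GetActorOfClass, rather than the controlled pawn, along its right and forward vectors.
; IA_camControle feeds its axes straight into the controller's yaw and pitch input.
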(event Input|EnhancedActionEvents|EnhancedInputActionIA_move
  (params (ActionValue :type Vector%202D%20Structure) (ElapsedSeconds :type Float%20%28double-precision%29) (TriggeredSeconds :type Float%20%28double-precision%29) (InputAction :type Input%20Action%20Object%20Reference :default "/Game/Le_Labyrinthe/IA/IA_move.IA_move"))
  ;[1 1 1] mouvement du joueur
  (:Triggered
    (bind _returnvalue (Actor|GetActorOfClass "/Game/Le_Labyrinthe/Blueprints/BP_FirstPersonCharacter.BP_FirstPersonCharacter_C"))
    (Pawn|Input|AddMovementInput _returnvalue (Transformation|GetActorRightVector _returnvalue) (.x ActionValue) false)
    (Pawn|Input|AddMovementInput _returnvalue (Transformation|GetActorForwardVector _returnvalue) (.y ActionValue) false)))

(event Input|EnhancedActionEvents|EnhancedInputActionIA_camControle
  (params (ActionValue :type Vector%202D%20Structure) (ElapsedSeconds :type Float%20%28double-precision%29) (TriggeredSeconds :type Float%20%28double-precision%29) (InputAction :type Input%20Action%20Object%20Reference :default "/Game/Le_Labyrinthe/IA/IA_camControle.IA_camControle"))
  ;[1 1 1] controlle de la cam
  (:Triggered
    (Class|PlayerController|AddYawInput (.x ActionValue))
    (Class|PlayerController|AddPitchInput (.y ActionValue))))

(event EventBeginPlay
  (bind _self self)
  (bind _returnvalue (PlayerController|LocalPlayerSubsystems|GetEnhancedInputLocalPlayerSubsystem _self))
  ;[1 1 1] ajout du mapping context
  (Utilities|IsValid _returnvalue
    (:Is%20Valid
      (Input|AddMappingContext _returnvalue "/Game/Le_Labyrinthe/IMC/IMC_Inputs.IMC_Inputs" 0 "(bIgnoreAllPressedKeysUntilRelease=True,bForceImmediately=False)"))))

(fn ConstructionScript)