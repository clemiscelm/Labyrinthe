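; Actor component that lets its owner toggle a switch ("interupteur") in the labyrinth game when the IA_interupteur input starts.
; It fires a short horizontal line trace from just above the owner's location along its facing direction, with debug drawing enabled.
; Any blocking hit on the trace channel calls InterupteurSwitch on BP_FirstPersonGameMode, without inspecting which actor was hit.
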(event Input|EnhancedActionEvents|EnhancedInputActionIA_interupteur
  (params (ActionValue :type Boolean) (ElapsedSeconds :type Float%20%28double-precision%29) (TriggeredSeconds :type Float%20%28double-precision%29) (InputAction :type Input%20Action%20Object%20Reference :default "/Game/Le_Labyrinthe/IA/IA_interupteur.IA_interupteur"))
  (bind _returnvalue (Components|GetOwner))
  (bind _returnvalue_2 (Transformation|GetActorLocation _returnvalue))
  (bind _returnvalue_3 (Transformation|GetActorRotation _returnvalue))
  (bind _returnvalue_4 (Math|Vector|GetForwardVector _returnvalue_3))
  (bind _returnvalue_5 (+ (.z _returnvalue_2) 1e+01))
  (bind (_x _y) (Class|KismetMathLibrary|BreakVector3f _returnvalue_4))
  (bind _returnvalue_6 (* (Math|Vector|MakeVector _x _y 0.0) 1e+02))
  ;[1 1 1] line trace
  (:Started
    (bind _returnvalue_7 (Collision|LineTraceByChannel (Math|Vector|MakeVector (.x _returnvalue_2) (.y _returnvalue_2) _returnvalue_5) (Math|Vector|MakeVector (+ (.x _returnvalue_2) (.x _returnvalue_6)) (+ (.y _returnvalue_2) (.y _returnvalue_6)) _returnvalue_5) "TraceTypeQuery3" false 0 "ForDuration"))
    (if _returnvalue_7
      ;[1 1 1] cast pour switch la variable torch
      (bind _asbp_first_person_game_mode (Utilities|Casting|CastToBP_FirstPersonGameMode (Game|GetGameMode)))
      (Default|InterupteurSwitch _asbp_first_person_game_mode))))